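; Player-controlled plane for the FirstMap practice level that flies forward on its own and fires rockets.
; Every Tick calls MoveForward, which adds full movement input along the Body component's forward vector; its DeltaSeconds parameter is unused.
; The Fire input spawns a BP_Rocekt_FirstMap_Pratice at the Arrow component's location with the Body's rotation, regardless of collision.
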(event EventBeginPlay)

(event Collision|EventActorBeginOverlap
  (params (OtherActor :type Actor%20Object%20Reference)))

(event EventTick
  (params (DeltaSeconds :type Float%20%28single-precision%29))
  (CallFunction|MoveForward 0.0))

(event Input|ActionEvents|InputActionFire
  (params (Key :type Key%20Structure :default "None"))
  (:Pressed
    (Game|SpawnActorfromClass "/Game/FirstMap_Pratice/Blueprints/BP_Rocekt_FirstMap_Pratice.BP_Rocekt_FirstMap_Pratice_C" (Math|Transform|MakeTransform (Transformation|GetWorldLocation (Variables|Default|GetArrow)) (Transformation|GetWorldRotation (Variables|Default|GetBody)) "1.000000,1.000000,1.000000") "AlwaysSpawn" "MultiplyWithRoot" 0 0)))

(fn ConstructionScript)

(fn MoveForward
  (params (DeltaSeconds :type Float%20%28double-precision%29))
  (Pawn|Input|AddMovementInput (Math|Vector|GetForwardVector (Variables|Default|GetBody)) 1.0 false))