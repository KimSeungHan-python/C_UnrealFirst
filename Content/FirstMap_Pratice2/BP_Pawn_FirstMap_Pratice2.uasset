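; BP_Pawn_FirstMap_Pratice2 is a player-controlled pawn that flies forward continuously, with a speed boost and rocket firing.
; Tick feeds its forward vector into FloatingPawnMovement and prints the current speed for debugging.
; Holding Boost scales the movement component's acceleration and max speed up from stored base values, and releasing restores them.
; Fire spawns a BP_Rocket_FirstMap_Pratice2 at the Arrow component's transform, with the pawn as owner and instigator.
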(event EventBeginPlay)

(event Collision|EventActorBeginOverlap
  (params (OtherActor :type Actor%20Object%20Reference)))

(event EventTick
  (params (DeltaSeconds :type Float%20%28single-precision%29))
  (Pawn|Input|AddMovementInput (Transformation|GetActorForwardVector) 1.0 false)
  (Development|PrintString (Utilities|String|ToString(Float) (Math|Vector|VectorLength (Variables|/Script/Engine.MovementComponent|GetVelocity (Variables|Default|GetFloatingPawnMovement))))))

(event Input|ActionEvents|InputActionFire
  (params (Key :type Key%20Structure :default "None"))
  (bind _self self)
  (:Pressed
    (Game|SpawnActorfromClass "/Game/FirstMap_Pratice2/BP_Rocket_FirstMap_Pratice2.BP_Rocket_FirstMap_Pratice2_C" (Transformation|GetWorldTransform (Variables|Default|GetArrow)) "AlwaysSpawn" "MultiplyWithRoot" _self _self)))

(event Input|ActionEvents|InputActionBoost
  (params (Key :type Key%20Structure :default "None"))
  (:Pressed
    (CallFunction|BoostStart))
  (:Released
    (CallFunction|BoostEnd)))

(fn ConstructionScript)

(fn BoostStart
  (bind _floatingpawnmovement (Variables|Default|GetFloatingPawnMovement))
  (Variables|/Script/Engine.FloatingPawnMovement|SetAcceleration _floatingpawnmovement (* (Variables|Default|GetAcceleration) 4.0))
  (Variables|/Script/Engine.FloatingPawnMovement|SetMaxSpeed _floatingpawnmovement (* (Variables|Default|GetMax%20Speed) 2.0)))

(fn BoostEnd
  (bind _floatingpawnmovement (Variables|Default|GetFloatingPawnMovement))
  (Variables|/Script/Engine.FloatingPawnMovement|SetAcceleration _floatingpawnmovement (Variables|Default|GetAcceleration))
  (Variables|/Script/Engine.FloatingPawnMovement|SetMaxSpeed _floatingpawnmovement (Variables|Default|GetMax%20Speed)))