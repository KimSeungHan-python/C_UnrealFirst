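; Rocket projectile actor that flies straight along its arrow and destroys itself on contact.
; Each tick it offsets itself without sweep along the Arrow component's forward vector, using the ProjectileMovement component's MaxSpeed scaled by delta time.
; It destroys itself when overlapping any actor except the first player's pawn, and a short lifespan set on BeginPlay removes it otherwise.
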(event EventBeginPlay
  (Actor|SetLifeSpan 3.0))

(event Collision|EventActorBeginOverlap
  (params (OtherActor :type Actor%20Object%20Reference))
  (if (not (== OtherActor (Game|Player|GetPlayerPawn 0)))
    (Actor|DestroyActor)))

(event EventTick
  (params (DeltaSeconds :type Float%20%28single-precision%29))
  (Transformation|AddActorWorldOffset (* DeltaSeconds (Variables|/Script/Engine.ProjectileMovementComponent|GetMaxSpeed (Variables|Default|GetProjectileMovement)) (Math|Vector|GetForwardVector (Variables|Default|GetArrow)))))

(fn ConstructionScript)