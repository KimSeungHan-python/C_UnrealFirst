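; BP_Pawn is a player-controlled flying pawn that constantly moves forward and can fire rockets.
; Tick adds movement input along the forward vector, scaled by a Boost value that the Boost action switches between full and half.
; Pitch and Roll axes rotate the pawn locally at a frame-rate-independent rate.
; The Fire action spawns BP_Rocket at the Arrow component's transform, with the pawn as owner and instigator.
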(event EventTick
  (params (DeltaSeconds :type Float%20%28single-precision%29))
  ;[0.15 0.15 0.15 0.5] 앞으로 전진
  (Pawn|Input|AddMovementInput (Transformation|GetActorForwardVector) (Variables|Default|GetBoost) false))

(event Input|ActionEvents|InputActionFire
  (params (Key :type Key%20Structure :default "None"))
  (bind _self self)
  (:Pressed
    (Game|SpawnActorfromClass "/Game/FirstMap/Blueprints/BP_Rocket.BP_Rocket_C" (Transformation|GetWorldTransform (Variables|Default|GetArrow)) "Undefined" "MultiplyWithRoot" _self _self)))

(event Input|ActionEvents|InputActionBoost
  (params (Key :type Key%20Structure :default "None"))
  ;[0.15 0.15 0.15 0.5] Boost
  (:Pressed
    (Variables|Default|SetBoost 1.0))
  (:Released
    (Variables|Default|SetBoost 0.5)))

(event Input|AxisEvents|InputAxisPitch
  (params (AxisValue :type Float%20%28single-precision%29))
  (Transformation|AddActorLocalRotation (Math|Rotator|MakeRotator 0.0 (* AxisValue 6e+01 (Utilities|Time|GetWorldDeltaSeconds)) 0.0) false false))

(event Input|AxisEvents|InputAxisRoll
  (params (AxisValue :type Float%20%28single-precision%29))
  (Transformation|AddActorLocalRotation (Math|Rotator|MakeRotator (* AxisValue 6e+01 (Utilities|Time|GetWorldDeltaSeconds)) 0.0 0.0) false false))

(fn ConstructionScript)