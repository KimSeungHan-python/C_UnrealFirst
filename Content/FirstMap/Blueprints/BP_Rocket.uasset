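; BP_Rocket is a projectile actor that explodes when its Box component begins overlapping any actor other than the first player's pawn.
; On that overlap it spawns the explosion effect and sound at its location, applies fixed damage credited to the first player controller, then destroys itself.
; BeginPlay sets a zero lifespan, so the rocket never expires by timer, and the graph contains no movement logic.
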(event OnComponentBeginOverlap(Box)
  (params (OverlappedComponent :type Primitive%20Component%20Object%20Reference) (OtherActor :type Actor%20Object%20Reference) (OtherComp :type Primitive%20Component%20Object%20Reference) (OtherBodyIndex :type Integer) (bFromSweep :type Boolean) (SweepResult :type Hit%20Result%20Structure%20%28by%20ref%29))
  (bind _returnvalue (Transformation|GetActorLocation))
  (if (not (== OtherActor (Game|Player|GetPlayerPawn 0)))
    (Niagara|SpawnSystematLocation "/Game/NiagaraExamples/FX_Explosions/NS_Explosion.NS_Explosion" _returnvalue)
    (Audio|SpawnSoundatLocation "/Game/FirstMap/Blueprints/Sounds/MS_Explosion.MS_Explosion" _returnvalue "0, 0, 0" 1.0 1.0 0.0 0 0)
    (Game|Damage|ApplyDamage OtherActor 1e+01 (Game|GetPlayerController 0) self)
    (Actor|DestroyActor)))

(event EventBeginPlay
  (Actor|SetLifeSpan 0.0))

(event Collision|EventActorBeginOverlap
  (params (OtherActor :type Actor%20Object%20Reference)))

(event EventTick
  (params (DeltaSeconds :type Float%20%28single-precision%29)))

(fn ConstructionScript)