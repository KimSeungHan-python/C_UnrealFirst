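; Moving target pawn whose death triggers game over in the first map.
; Every tick it feeds movement input along its Arrow component's forward vector.
; Any damage it receives reduces Hp; at zero or below it destroys itself and calls GameOver on the BP_GM game mode.
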(event EventBeginPlay)

(event EventTick
  (params (DeltaSeconds :type Float%20%28single-precision%29))
  (Pawn|Input|AddMovementInput (* (Math|Vector|GetForwardVector (Variables|Default|GetArrow)) 5e+01) 1.0 false))

(event Game|Damage|EventAnyDamage
  (params (Damage :type Float%20%28single-precision%29) (DamageType :type Damage%20Type%20Object%20Reference) (InstigatedBy :type Controller%20Object%20Reference) (DamageCauser :type Actor%20Object%20Reference))
  (bind _output_get (Variables|Default|SetHp (- (Variables|Default|GetHp) Damage)))
  (if (<= _output_get 0.0)
    (Actor|DestroyActor)
    (bind _asbp_gm (Utilities|Casting|CastToBP_GM (Game|GetGameMode)))
    (Default|GameOver _asbp_gm)))

(fn ConstructionScript)